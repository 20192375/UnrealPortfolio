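; Red GrabPack hand actor that snaps the player's right hand onto red hand scanners, doors, power receivers and power sources.
; Each event nudges the hand mesh by hardcoded offsets, attaches it to the target referenced on BP_Character1, and points the CableRightHand end at it.
; Scanner events also toggle RightHandAttached, with a finish event applying reverse offsets.
; Door and power events play looping hand animations.
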(event `AttachHandToScanner`
  (bind _sk_grabpackhand_defaultoriginalscrewed_red (`self.SK_GrabpackHand_DefaultOriginalScrewed_Red`))
  (bind _sk_grabpackhand_defaultoriginalscrewed_red_2 (`self.SK_GrabpackHand_DefaultOriginalScrewed_Red`))
  (bind (_relativerotation_roll _relativerotation_pitch _relativerotation_yaw) (`KismetMathLibrary.BreakRotator` (`SceneComponent.RelativeRotation` _sk_grabpackhand_defaultoriginalscrewed_red)))
  (bind (_relativelocation_x _relativelocation_y _relativelocation_z) (`KismetMathLibrary.BreakVector` (`SceneComponent.RelativeLocation` _sk_grabpackhand_defaultoriginalscrewed_red)))
  ;[1 0 0 0.8] RedHandScanner
  (`|ExecutionSequence`
    (:`then_0`
      (bind _asbp_character_1 (cast `/Game/ThirdPerson/Blueprints/BP_Character1` (`GameplayStatics.GetPlayerCharacter` 0)))
      (`SceneComponent.K2_AddRelativeRotation` _sk_grabpackhand_defaultoriginalscrewed_red_2 (`KismetMathLibrary.MakeRotator` _relativerotation_roll _relativerotation_pitch (- _relativerotation_yaw 0.0)) false false)
      (`SceneComponent.K2_AddRelativeLocation` _sk_grabpackhand_defaultoriginalscrewed_red_2 (`KismetMathLibrary.MakeVector` (- _relativelocation_x 3.0) (+ _relativelocation_y 16.0) (+ _relativelocation_z 21.0)) false false)
      (`SceneComponent.SetRelativeScale3D` _sk_grabpackhand_defaultoriginalscrewed_red_2 (0.35 0.35 0.35))
      (`|ExecutionSequence`
        (:`then_0`
          (`SceneComponent.K2_AttachToComponent` _sk_grabpackhand_defaultoriginalscrewed_red_2 (`/Game/Blueprints/Mechanics/BlueHandScanner/BP_HandScannerRED.HandScannerButtonModel` (`/Game/ThirdPerson/Blueprints/BP_Character1.BP_RedHandScannerRef` _asbp_character_1)) "None" "KeepRelative" "KeepRelative" "KeepRelative" true))
        (:`then_1`
          (bind _asbp_character_1_2 (cast `/Game/ThirdPerson/Blueprints/BP_Character1` (`GameplayStatics.GetPlayerCharacter` 0)))
          (set `/Game/ThirdPerson/Blueprints/BP_Character1.RightHandAttached?` true _asbp_character_1_2)
          (`CableComponent.SetAttachEndToComponent` (`/Game/ThirdPerson/Blueprints/BP_Character1.CableRightHand` _asbp_character_1_2) (`self.SK_GrabpackHand_DefaultOriginalScrewed_Red`) "None"))))))

(event `AttachHandToScanner_Finished`
  (bind _sk_grabpackhand_defaultoriginalscrewed_red (`self.SK_GrabpackHand_DefaultOriginalScrewed_Red`))
  (bind _sk_grabpackhand_defaultoriginalscrewed_red_2 (`self.SK_GrabpackHand_DefaultOriginalScrewed_Red`))
  (bind (_relativerotation_roll _relativerotation_pitch _relativerotation_yaw) (`KismetMathLibrary.BreakRotator` (`SceneComponent.RelativeRotation` _sk_grabpackhand_defaultoriginalscrewed_red_2)))
  (bind (_relativelocation_x _relativelocation_y _relativelocation_z) (`KismetMathLibrary.BreakVector` (`SceneComponent.RelativeLocation` _sk_grabpackhand_defaultoriginalscrewed_red_2)))
  ;[1 0 0 0.8] RedHandScanner
  (bind _returnvalue (`GameplayStatics.GetActorOfClass` "/Game/Blueprints/Mechanics/BlueHandScanner/BP_HandScannerRED.BP_HandScannerRED_C"))
  (`SceneComponent.K2_AddRelativeRotation` _sk_grabpackhand_defaultoriginalscrewed_red (`KismetMathLibrary.MakeRotator` _relativerotation_roll _relativerotation_pitch (+ _relativerotation_yaw 360.0)) false false)
  (`SceneComponent.K2_AddRelativeLocation` _sk_grabpackhand_defaultoriginalscrewed_red (`KismetMathLibrary.MakeVector` (+ _relativelocation_x 3.0) (- _relativelocation_y 16.0) (- _relativelocation_z 21.0)) false false)
  (`|ExecutionSequence`
    (:`then_0`
      (`SceneComponent.K2_AttachToComponent` _sk_grabpackhand_defaultoriginalscrewed_red (`/Game/Blueprints/Mechanics/BlueHandScanner/BP_HandScannerRED.HandScannerButtonModel` _returnvalue) "None" "KeepRelative" "KeepRelative" "KeepRelative" true))
    (:`then_1`
      (bind _asbp_character_1 (cast `/Game/ThirdPerson/Blueprints/BP_Character1` (`GameplayStatics.GetPlayerCharacter` 0)))
      (set `/Game/ThirdPerson/Blueprints/BP_Character1.RightHandAttached?` false _asbp_character_1)
      (`CableComponent.SetAttachEndToComponent` (`/Game/ThirdPerson/Blueprints/BP_Character1.CableRightHand` _asbp_character_1) (`self.SK_GrabpackHand_DefaultOriginalScrewed_Red`) "None"))))

(event `AttachHandToDoor`
  (bind _sk_grabpackhand_defaultoriginalscrewed_red (`self.SK_GrabpackHand_DefaultOriginalScrewed_Red`))
  (bind _sk_grabpackhand_defaultoriginalscrewed_red_2 (`self.SK_GrabpackHand_DefaultOriginalScrewed_Red`))
  (bind (_relativerotation_roll _relativerotation_pitch _relativerotation_yaw) (`KismetMathLibrary.BreakRotator` (`SceneComponent.RelativeRotation` _sk_grabpackhand_defaultoriginalscrewed_red_2)))
  (bind (_relativelocation_x _relativelocation_y _relativelocation_z) (`KismetMathLibrary.BreakVector` (`SceneComponent.RelativeLocation` _sk_grabpackhand_defaultoriginalscrewed_red_2)))
  ;[1 0.991 0] AttachHandToDoor
  (bind _asbp_character_1 (cast `/Game/ThirdPerson/Blueprints/BP_Character1` (`GameplayStatics.GetPlayerCharacter` 0)))
  (`SceneComponent.K2_AddRelativeRotation` _sk_grabpackhand_defaultoriginalscrewed_red (`KismetMathLibrary.MakeRotator` _relativerotation_roll _relativerotation_pitch _relativerotation_yaw) false false)
  (`SceneComponent.K2_AddRelativeLocation` _sk_grabpackhand_defaultoriginalscrewed_red (`KismetMathLibrary.MakeVector` (+ _relativelocation_x 95.0) (+ _relativelocation_y 17.0) (+ _relativelocation_z 105.0)) false false)
  (`SkeletalMeshComponent.PlayAnimation` (`self.SK_GrabpackHand_DefaultOriginalScrewed_Red`) "/Game/Hand/SK_Hand_Grab_GrabHook_Montage.SK_Hand_Grab_GrabHook_Montage" true)
  (`SceneComponent.K2_AttachToComponent` (`self.SK_GrabpackHand_DefaultOriginalScrewed_Red`) (`/Game/Blueprints/Mechanics/Doors/BP_Door.DoorMesh` (`/Game/ThirdPerson/Blueprints/BP_Character1.BP_DoorRef` _asbp_character_1)) "None" "KeepRelative" "KeepRelative" "KeepRelative" true)
  (bind _asbp_character_1_2 (cast `/Game/ThirdPerson/Blueprints/BP_Character1` (`GameplayStatics.GetPlayerCharacter` 0)))
  (`CableComponent.SetAttachEndToComponent` (`/Game/ThirdPerson/Blueprints/BP_Character1.CableRightHand` _asbp_character_1_2) (`self.SK_GrabpackHand_DefaultOriginalScrewed_Red`) "None"))

(event `AttachHandToPowerReceiver`
  (bind _sk_grabpackhand_defaultoriginalscrewed_red (`self.SK_GrabpackHand_DefaultOriginalScrewed_Red`))
  (bind _sk_grabpackhand_defaultoriginalscrewed_red_2 (`self.SK_GrabpackHand_DefaultOriginalScrewed_Red`))
  (bind (_relativerotation_roll _relativerotation_pitch _relativerotation_yaw) (`KismetMathLibrary.BreakRotator` (`SceneComponent.RelativeRotation` _sk_grabpackhand_defaultoriginalscrewed_red_2)))
  (bind (_relativelocation_x _relativelocation_y _relativelocation_z) (`KismetMathLibrary.BreakVector` (`SceneComponent.RelativeLocation` _sk_grabpackhand_defaultoriginalscrewed_red_2)))
  ;[0 0.2344 0.1543] AttachHandToPowerReceiver
  (bind _asbp_character_1 (cast `/Game/ThirdPerson/Blueprints/BP_Character1` (`GameplayStatics.GetPlayerCharacter` 0)))
  (`SceneComponent.K2_AddRelativeRotation` _sk_grabpackhand_defaultoriginalscrewed_red (`KismetMathLibrary.MakeRotator` _relativerotation_roll _relativerotation_pitch _relativerotation_yaw) false false)
  (`SceneComponent.K2_AddRelativeLocation` _sk_grabpackhand_defaultoriginalscrewed_red (`KismetMathLibrary.MakeVector` _relativelocation_x (+ _relativelocation_y 15.0) (- _relativelocation_z 20.0)) false false)
  (`SkeletalMeshComponent.PlayAnimation` (`self.SK_GrabpackHand_DefaultOriginalScrewed_Red`) "/Game/Hand/SK_Grabpack_HandBlue_Sphere.SK_Grabpack_HandBlue_Sphere" true)
  (`SceneComponent.K2_AttachToComponent` (`self.SK_GrabpackHand_DefaultOriginalScrewed_Red`) (`/Game/Blueprints/Mechanics/Poles/BP_PowerReceiver.ReceiverMesh` (`/Game/ThirdPerson/Blueprints/BP_Character1.BP_PowerReceiverRef` _asbp_character_1)) "None" "KeepRelative" "KeepRelative" "KeepRelative" true)
  (bind _asbp_character_1_2 (cast `/Game/ThirdPerson/Blueprints/BP_Character1` (`GameplayStatics.GetPlayerCharacter` 0)))
  (`CableComponent.SetAttachEndToComponent` (`/Game/ThirdPerson/Blueprints/BP_Character1.CableRightHand` _asbp_character_1_2) (`self.SK_GrabpackHand_DefaultOriginalScrewed_Red`) "None"))

(event `AttachHandToPowerSource`
  (bind _sk_grabpackhand_defaultoriginalscrewed_red (`self.SK_GrabpackHand_DefaultOriginalScrewed_Red`))
  (bind _sk_grabpackhand_defaultoriginalscrewed_red_2 (`self.SK_GrabpackHand_DefaultOriginalScrewed_Red`))
  (bind (_relativerotation_roll _relativerotation_pitch _relativerotation_yaw) (`KismetMathLibrary.BreakRotator` (`SceneComponent.RelativeRotation` _sk_grabpackhand_defaultoriginalscrewed_red)))
  (bind (_relativelocation_x _relativelocation_y _relativelocation_z) (`KismetMathLibrary.BreakVector` (`SceneComponent.RelativeLocation` _sk_grabpackhand_defaultoriginalscrewed_red)))
  ;[0 0.08854 0.05828] AttachHandToPowerSource
  (bind _asbp_character_1 (cast `/Game/ThirdPerson/Blueprints/BP_Character1` (`GameplayStatics.GetPlayerCharacter` 0)))
  (`SceneComponent.K2_AddRelativeRotation` _sk_grabpackhand_defaultoriginalscrewed_red_2 (`KismetMathLibrary.MakeRotator` _relativerotation_roll _relativerotation_pitch _relativerotation_yaw) false false)
  (`SceneComponent.K2_AddRelativeLocation` _sk_grabpackhand_defaultoriginalscrewed_red_2 (`KismetMathLibrary.MakeVector` _relativelocation_x (+ _relativelocation_y 36.0) (+ _relativelocation_z 43.0)) false false)
  (`SkeletalMeshComponent.PlayAnimation` (`self.SK_GrabpackHand_DefaultOriginalScrewed_Red`) "/Game/Hand/SK_Grabpack_HandBlue_Sphere.SK_Grabpack_HandBlue_Sphere" true)
  (`SceneComponent.K2_AttachToComponent` (`self.SK_GrabpackHand_DefaultOriginalScrewed_Red`) (`/Game/Blueprints/Mechanics/Poles/BP_PowerSource.SourceMesh` (`/Game/ThirdPerson/Blueprints/BP_Character1.BP_PowerSourceRef` _asbp_character_1)) "None" "KeepRelative" "KeepRelative" "KeepRelative" true)
  (bind _asbp_character_1_2 (cast `/Game/ThirdPerson/Blueprints/BP_Character1` (`GameplayStatics.GetPlayerCharacter` 0)))
  (`CableComponent.SetAttachEndToComponent` (`/Game/ThirdPerson/Blueprints/BP_Character1.CableRightHand` _asbp_character_1_2) (`self.SK_GrabpackHand_DefaultOriginalScrewed_Red`) "None"))

(fn `UserConstructionScript`)