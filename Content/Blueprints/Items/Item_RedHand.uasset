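; Red Hand item actor that offers a pickup prompt when the player character is near.
; On BeginPlay it destroys itself if the game instance's save data already has the Red Hand, otherwise prints a debug message.
; Overlap by BP_Character1 shows an ItemGetUse widget and passes the item to the character via OverlapForGetItemMessage.
; End overlap removes the widget and sends that message without an item.
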(event `self.ReceiveBeginPlay`
  (bind _asbp_gi (cast `/Game/Blueprints/Core/BP_GI` (`GameplayStatics.GetGameInstance`)))
  (if (`/Game/Blueprints/Core/BP_SaveGame.HasRedHand` (`/Game/Blueprints/Core/BP_GI.SaveRef` _asbp_gi))
    (`self.K2_DestroyActor`)
    (else
      (`KismetSystemLibrary.PrintString` "Hello, RED Here"))))

(event `self.ReceiveActorBeginOverlap`
  (params (OtherActor :type "Actor Object Reference"))
  (bind _asbp_character_1 (cast `/Game/ThirdPerson/Blueprints/BP_Character1` OtherActor))
  (bind _returnvalue (`|CreateWidget` "/Game/UI/ItemGetUse.ItemGetUse_C"))
  (`UserWidget.AddToViewport` _returnvalue 0)
  (`Widget.SetVisibility` (`/Game/UI/ItemGetUse.Pick` _returnvalue) "Visible")
  (message `/Game/Blueprints/Items/BPI_InteractItem.OverlapForGetItem` _asbp_character_1 self))

(event `self.ReceiveActorEndOverlap`
  (params (OtherActor :type "Actor Object Reference"))
  (`Widget.RemoveFromParent` (stale `self.ReceiveActorBeginOverlap` _returnvalue))
  (message `/Game/Blueprints/Items/BPI_InteractItem.OverlapForGetItem` OtherActor null))

(fn `UserConstructionScript`)