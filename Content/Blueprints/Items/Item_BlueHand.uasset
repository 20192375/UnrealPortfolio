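; Blue Hand world pickup that offers a pick-up prompt when an actor overlaps it.
; On BeginPlay it reads the save in BP_GI and destroys itself if the Blue Hand is already owned.
; Overlap begin creates an ItemGetUse widget showing Pick and passes itself via OverlapForGetItemMessage; overlap end removes the widget and resends the message without an item.
; The actual pickup logic is not in this Blueprint.
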(event `self.ReceiveBeginPlay`
  (bind _asbp_gi (cast `/Game/Blueprints/Core/BP_GI` (`GameplayStatics.GetGameInstance`)))
  (if (`/Game/Blueprints/Core/BP_SaveGame.HasBlueHand` (`/Game/Blueprints/Core/BP_GI.SaveRef` _asbp_gi))
    (`KismetSystemLibrary.PrintString` "BLUEBYE!")
    (`self.K2_DestroyActor`)))

(event `self.ReceiveActorBeginOverlap`
  (params (OtherActor :type "Actor Object Reference"))
  (bind _returnvalue (`|CreateWidget` "/Game/UI/ItemGetUse.ItemGetUse_C"))
  (`UserWidget.AddToViewport` _returnvalue 0)
  (`Widget.SetVisibility` (`/Game/UI/ItemGetUse.Pick` _returnvalue) "Visible")
  (message `/Game/Blueprints/Items/BPI_InteractItem.OverlapForGetItem` OtherActor self))

(event `self.ReceiveActorEndOverlap`
  (params (OtherActor :type "Actor Object Reference"))
  (`Widget.RemoveFromParent` (stale `self.ReceiveActorBeginOverlap` _returnvalue))
  (message `/Game/Blueprints/Items/BPI_InteractItem.OverlapForGetItem` OtherActor null))

(fn `UserConstructionScript`)