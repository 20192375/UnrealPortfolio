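; HugeBox is an item that falls after two hands have attached and both let go, apparently as part of a HuggyWuggy encounter.
; HandAttached and HandLeft count hands; release triggers Drop only if HuggyWuggy's Ultimatum is off, also clearing its CanCatch flag.
; Drop messages RushActor, then the MoveBox timeline lerps the box toward a hard-coded position and tilt before enabling physics simulation.
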(event `self.ReceiveActorBeginOverlap`
  (params (OtherActor :type "Actor Object Reference")))

(event `HandAttached`
  (bind _result (`/Engine/EditorBlueprintResources/StandardMacros.IncrementInt` (`self.attachedHand`))
    (:`  `
      (bind _output_get (set `self.attachedHand` _result))
      (set `self.ReadytoDrop` (>= _output_get 2)))))

(event `HandLeft`
  (bind _attachedhand (`self.attachedHand`))
  (bind _result (`/Engine/EditorBlueprintResources/StandardMacros.DecrementInt` _attachedhand)
    (:`  `
      (set `self.attachedHand` _result)
      (if (== _attachedhand 0)
        (if (`self.ReadytoDrop`)
          (bind _returnvalue (`GameplayStatics.GetActorOfClass` "/Game/Characters/HW/glb/HuggyWuggy.HuggyWuggy_C"))
          (if (not (`/Game/Characters/HW/glb/HuggyWuggy.Ultimatum` _returnvalue))
            (set `/Game/Characters/HW/glb/HuggyWuggy.CanCatch` false _returnvalue)
            (`self.Drop`)))))))

(event `Drop`
  (bind (_returnvalue_x _returnvalue_y _returnvalue_z) (`KismetMathLibrary.BreakVector` (`self.K2_GetActorLocation`)))
  (message `/Game/Blueprints/Items/BPI_Box.RushToBox` (`self.RushActor`))
  (`KismetSystemLibrary.PrintString` "GOOD BYE!")
  (bind (_direction _lerp) (`Timeline|MoveBox` :!via `PlayFromStart`)
    (:`Update`
      (`self.K2_SetActorTransform` (`KismetMathLibrary.MakeTransform` (`KismetMathLibrary.VLerp` (`KismetMathLibrary.MakeVector` _returnvalue_x _returnvalue_y _returnvalue_z) (`KismetMathLibrary.MakeVector` _returnvalue_x -1210.0 857.0) _lerp) (`KismetMathLibrary.RLerp` (struct) (struct :`Roll` -60.0) _lerp) (6.0 6.0 6.0))))
    (:`Finished`
      (`PrimitiveComponent.SetSimulatePhysics` (`self.Box`) true))))

(fn `UserConstructionScript`)