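; BP_PowerSource is a puzzle power node that links a pole to a cable.
; Its FillCable event proceeds only if the player is BP_Character1, then checks whether LinkedPole is powered.
; If so, it marks itself powered and, when LinkedCable is valid, sets that cable filling and prints a puzzle-completed message.
; Nothing in this Blueprint calls FillCable, and its default events are unused.
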(event `FillCable`
  (bind _linked_cable (`self.Linked Cable`))
  (cast `/Game/ThirdPerson/Blueprints/BP_Character1` (`GameplayStatics.GetPlayerCharacter` 0))
  (if (`/Game/Blueprints/Mechanics/Poles/BP_PuzzlePole.IsPowered?` (`self.Linked Pole`))
    (set `self.IsPowered` true)
    (`/Engine/EditorBlueprintResources/StandardMacros.IsValid` _linked_cable
      (:`Is Valid`
        (set `/Game/Blueprints/BP_Cable/BP_Cable.IsFilling?` true _linked_cable)
        (`KismetSystemLibrary.PrintString` "Flling Cable. Puzzle is Completed")))
    (else
      (`KismetSystemLibrary.PrintString` "NOT Powered"))))

(fn `UserConstructionScript`)