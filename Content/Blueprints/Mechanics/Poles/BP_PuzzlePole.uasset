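; BP_PuzzlePole is a puzzle pole actor whose active logic only reapplies its basic material to the pole mesh every Tick.
; Its player collision overlap events are empty.
; An unwired branch would clear IsPowered and play a discharge sound when its power source is unpowered and either of the third-person character's hands is attached to a power receiver.
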(event `self.ReceiveTick`
  (params (DeltaSeconds :type "Float (single-precision)"))
  (`PrimitiveComponent.SetMaterial` (`self.PoleMesh`) 0 "/Game/Meshes/Gameplay/PolePuzzles/source/MI_PuzzlePole_Basic.MI_PuzzlePole_Basic"))

(event `self.CollisionPlayer.OnComponentBeginOverlap`
  (params (OverlappedComponent :type "PrimitiveComponent Object Reference") (OtherActor :type "Actor Object Reference") (OtherComp :type "PrimitiveComponent Object Reference") (OtherBodyIndex :type Integer) (bFromSweep :type Boolean) (SweepResult :type "HitResult Structure (by ref)")))

(event `self.CollisionPlayer.OnComponentEndOverlap`
  (params (OverlappedComponent :type "PrimitiveComponent Object Reference") (OtherActor :type "Actor Object Reference") (OtherComp :type "PrimitiveComponent Object Reference") (OtherBodyIndex :type Integer)))

(fn `UserConstructionScript`)