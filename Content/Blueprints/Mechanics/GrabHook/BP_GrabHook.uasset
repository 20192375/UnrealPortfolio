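; BP_GrabHook is a grab hook actor that serves as a target for the GrabPack's grapple.
; On BeginPlay it stores a Location point 350 units below its own position.
; A Grappled event plays the hand launch sound, and paired events switch its four collision components on or off.
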(event `self.ReceiveBeginPlay`
  (bind (_returnvalue_x _returnvalue_y _returnvalue_z) (`KismetMathLibrary.BreakVector` (`self.K2_GetActorLocation`)))
  (set `self.Location` (`KismetMathLibrary.MakeVector` _returnvalue_x _returnvalue_y (- _returnvalue_z 350.0))))

(event `Grappled`
  (`GameplayStatics.PlaySound2D` "/Game/Sounds/Grabpack/SW_Grabpack_HandLaunch_02.SW_Grabpack_HandLaunch_02" 1.0 1.0 0.0 null null))

(event `SetCollisionsOn`
  (`PrimitiveComponent.SetCollisionEnabled` (`self.Collision2`) "QueryAndPhysics")
  (`PrimitiveComponent.SetCollisionEnabled` (`self.Collision3`) "QueryAndPhysics")
  (`PrimitiveComponent.SetCollisionEnabled` (`self.Collision4`) "QueryAndPhysics")
  (`PrimitiveComponent.SetCollisionEnabled` (`self.Collision1`) "QueryAndPhysics"))

(event `SetCollisionsOff`
  (`PrimitiveComponent.SetCollisionEnabled` (`self.Collision1`) "NoCollision")
  (`PrimitiveComponent.SetCollisionEnabled` (`self.Collision4`) "NoCollision")
  (`PrimitiveComponent.SetCollisionEnabled` (`self.Collision3`) "NoCollision")
  (`PrimitiveComponent.SetCollisionEnabled` (`self.Collision2`) "NoCollision"))

(fn `UserConstructionScript`)