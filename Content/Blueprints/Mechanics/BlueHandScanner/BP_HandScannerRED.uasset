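; Red hand scanner actor that, while powered, runs a scan and notifies its linked ActorToOpen when it finishes.
; PlayAnim_Scanner starts sounds and a timeline that stretches the progress bar, calling CancelAnim to reset if power is absent.
; Poweron counts inserted batteries toward a required total, while any PowerOff call cuts power.
; Powered and unpowered states currently apply the same button material.
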(event `PlayAnim_Scanner`
  ;[1 0 0] MainLogic
  (`|ExecutionSequence`
    (:`then_0`
      (bind (_direction _alphanew) (`Timeline|TL` :!via `PlayFromStart`)
        (:`Update`
          (if (`self.IsPowered?`)
            (`SceneComponent.SetRelativeScale3D` (`self.HandScannerBar`) (`KismetMathLibrary.MakeVector` _alphanew 1.0 1.0))
            (else
              (`self.CancelAnim`))))
        (:`Finished`
          (set `self.IsRedScanningFinished` true)
          (`SceneComponent.SetRelativeScale3D` (`self.HandScannerBar`) (2.028777 1.0 1.0))
          (`GameplayStatics.PlaySoundAtLocation` "/Game/Sounds/BlueScanner/SW_Keypad_Unlock.SW_Keypad_Unlock" (`self.K2_GetActorLocation`) (struct) 1.0 1.0 0.0 null null null null)
          (message `/Game/Blueprints/Mechanics/BlueHandScanner/BPI_HandScannerEvent.ScanningFinished` (`self.Actor To Open`)))))
    (:`then_1`
      (bind _returnvalue (`AddComponent|NODE_AddAudioComponent-0`))
      (bind _output_get (set `self.SW_HandScanning_Sound` _returnvalue))
      (`AudioComponent.Play` _output_get 0.0))
    (:`then_2`
      (`GameplayStatics.PlaySoundAtLocation` "/Game/Sounds/Grabpack/SW_Grabpack_HandLaunch_02.SW_Grabpack_HandLaunch_02" (`self.K2_GetActorLocation`) (struct) 1.0 1.0 0.0 null null null null))))

(event `CancelAnim`
  ;[1 0 0] MainLogic
  (set `self.IsRedScanningFinished` false)
  (`KismetSystemLibrary.PrintString` "CancelledScanning")
  (`TimelineComponent.Stop` (`self.TL`))
  (`KismetSystemLibrary.Delay` 0.1)
  (`SceneComponent.SetRelativeScale3D` (`self.HandScannerBar`) (0.007318 1.0 1.0))
  (`AudioComponent.Stop` (`self.SW_HandScanning_Sound`)))

(event `self.PowerOn`
  (bind _howmanybatteriesinserted_ (`self.HowManyBatteriesInserted?`))
  ;[0.179 0.5114 1] PowerByBattery
  (`/Engine/EditorBlueprintResources/StandardMacros.IncrementInt` _howmanybatteriesinserted_
    (:`  `
      (if (>= _howmanybatteriesinserted_ (`self.HowManyBatteriesNeedToPower?`))
        (set `self.IsPowered?` true)
        (`PrimitiveComponent.SetMaterial` (`self.HandScannerButtonModel`) 0 "/Game/Materials/Gameplay/HandScanner/M_RedHand_Normal1.M_RedHand_Normal1")))))

(event `self.PowerOff`
  (bind _howmanybatteriesinserted_ (`self.HowManyBatteriesInserted?`))
  ;[0.179 0.5114 1] PowerByBattery
  (`/Engine/EditorBlueprintResources/StandardMacros.DecrementInt` _howmanybatteriesinserted_
    (:`  `
      (if (>= _howmanybatteriesinserted_ (`self.HowManyBatteriesNeedToPower?`))
        _
        (else
          _))
      (set `self.IsPowered?` false)
      (`PrimitiveComponent.SetMaterial` (`self.HandScannerButtonModel`) 0 "/Game/Materials/Gameplay/HandScanner/M_RedHand_Normal1.M_RedHand_Normal1"))))

(fn `UserConstructionScript`
  (bind _handscannerbuttonmodel (`self.HandScannerButtonModel`))
  (if (`self.IsPowered?`)
    (`PrimitiveComponent.SetMaterial` _handscannerbuttonmodel 0 "/Game/Materials/Gameplay/HandScanner/M_RedHand_Normal1.M_RedHand_Normal1")
    (else
      (`PrimitiveComponent.SetMaterial` _handscannerbuttonmodel 0 "/Game/Materials/Gameplay/HandScanner/M_RedHand_Normal1.M_RedHand_Normal1"))))