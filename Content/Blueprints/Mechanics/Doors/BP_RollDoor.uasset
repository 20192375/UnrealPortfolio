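; Roll-up metal door that slides vertically with sound, triggered by hand scans, a lever or inserted batteries.
; ToggleDoor flips the state behind a busy flag, animates the mesh with MoveComponentTo and records DoorNumber on the player character.
; BeginPlay toggles doors numbered within the GameInstance's saved opened count; PowerOff decrements batteries and calls DoorClose regardless of threshold.
; The construction script sets colour by DoorType and the initial open or closed position.
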(event `self.ReceiveBeginPlay`
  (bind _asbp_gi (cast `/Game/Blueprints/Core/BP_GI` (`GameplayStatics.GetGameInstance`)))
  (if (<= (`self.DoorNumber`) (`/Game/Blueprints/Core/BP_SaveGame.Count_OpenedDoor` (`/Game/Blueprints/Core/BP_GI.SaveRef` _asbp_gi)))
    (`self.ToggleDoor`)))

(event `ToggleDoor`
  (bind _playercache (`self.PlayerCache`))
  (if (not (`self.IsOpeningDoor`)) :!label _label
    (set `self.IsOpeningDoor` true)
    (bind _output_get (set `self.IsDoorOpened` (not (`self.IsDoorOpened`))))
    (`/Engine/EditorBlueprintResources/StandardMacros.IsValid` _playercache
      (:`Is Valid`
        _)
      (:`Is Not Valid`
        (bind _asbp_character_1 (cast `/Game/ThirdPerson/Blueprints/BP_Character1` (`GameplayStatics.GetPlayerCharacter` 0)))
        (set `self.PlayerCache` _asbp_character_1)))
    (bind _output_get_2 (set `/Game/ThirdPerson/Blueprints/BP_Character1.Count_SaveOpenDoor` (`self.DoorNumber`) _playercache))
    (`KismetSystemLibrary.PrintString` (`KismetStringLibrary.Conv_IntToString` _output_get_2))
    (`GameplayStatics.PlaySoundAtLocation` "/Game/Sounds/Doors/Metal/SW_Door_Metal_AutoOpen_Cue.SW_Door_Metal_AutoOpen_Cue" (`self.K2_GetActorLocation`) (struct) 1.0 1.0 0.0 null null null null)
    (`KismetSystemLibrary.MoveComponentTo` (`self.DoorMesh`) (`KismetMathLibrary.MakeVector` 1.275385 0.0 (`KismetMathLibrary.SelectFloat` (`self.DoorMaxLocation`) -1e-06 _output_get)) (`KismetMathLibrary.MakeRotator` 0.0) false false 1.0 true)
    (set `self.IsOpeningDoor` false)))

(event `/Game/Blueprints/Mechanics/BlueHandScanner/BPI_HandScannerEvent.ScanningFinished`
  (bind _result (`/Engine/EditorBlueprintResources/StandardMacros.IncrementInt` (`self.Hands`))
    (:`  `
      (if (>= _result (`self.HandsNeeded`))
        (goto _label)))))

(event `/Game/Blueprints/Mechanics/Lever/BPI_LeverEvents.LeverOpen`
  (goto _label))

(event `/Game/Blueprints/Mechanics/Battery/BPI_BatteryEvent.Door_SetDoorOpened`
  (set `self.IsDoorOpened` true))

(event `DoorClose`
  (if (`self.IsDoorOpened`)
    (if (not (`self.IsOpeningDoor`))
      (set `self.IsOpeningDoor` true)
      (`GameplayStatics.PlaySoundAtLocation` "/Game/Sounds/Doors/Metal/SW_Door_Metal_AutoOpen_Cue.SW_Door_Metal_AutoOpen_Cue" (`self.K2_GetActorLocation`) (struct) 1.0 1.0 0.0 null null null null)
      (`KismetSystemLibrary.MoveComponentTo` (`self.DoorMesh`) (`KismetMathLibrary.MakeVector` 1.275385 0.0 (`KismetMathLibrary.SelectFloat` 252.822249 -1e-06)) (`KismetMathLibrary.MakeRotator` 0.0) false false 1.0 true)
      (set `self.IsDoorOpened` false)
      (set `self.IsOpeningDoor` false))))

(event `/Game/Blueprints/Mechanics/Battery/BPI_BatteryEvent.Door_SetDoorClosed`
  (set `self.IsDoorOpened` false))

(event `/Game/Blueprints/BP_Cable/BPI_PowerNew.PowerOn`
  (bind _howmanybatteriesinserted_ (`self.HowManyBatteriesInserted?`))
  (bind _result (`/Engine/EditorBlueprintResources/StandardMacros.IncrementInt` _howmanybatteriesinserted_)
    (:`  `
      (`KismetSystemLibrary.PrintString` (`KismetStringLibrary.Conv_IntToString` _result) true true (struct :`R` 0.901093 :`G` 1.0 :`A` 1.0))
      (if (>= _howmanybatteriesinserted_ (`self.HowManyBatteriesNeedToPower?`))
        (`self.ToggleDoor`)))))

(event `/Game/Blueprints/BP_Cable/BPI_PowerNew.PowerOff`
  (bind _howmanybatteriesinserted_ (`self.HowManyBatteriesInserted?`))
  (`|ExecutionSequence`
    (:`then_0`
      (`/Engine/EditorBlueprintResources/StandardMacros.DecrementInt` _howmanybatteriesinserted_
        (:`  `
          (if (not (>= _howmanybatteriesinserted_ (`self.HowManyBatteriesNeedToPower?`)))
            (`self.DoorClose` :!label _label_2)))))
    (:`then_1`
      (goto _label_2))))

(fn `UserConstructionScript`
  (`|ExecutionSequence`
    (:`then_0`
      (for _array_element (`|MakeArray` (`self.FrameMesh`) (`self.DoorMesh`))
        (`PrimitiveComponent.SetMaterial` _array_element 0 (select `int` (`self.DoorType`) :`0` "/Game/Textures/Kits/RollDoor/T_RollUpDoor_C_Blue_DIF_Mat.T_RollUpDoor_C_Blue_DIF_Mat" :`1` "/Game/Textures/Kits/RollDoor/T_RollUpDoor_C_Red_DIF_Mat.T_RollUpDoor_C_Red_DIF_Mat" :`2` "/Game/Textures/Kits/RollDoor/T_RollUpDoor_C_Yellow_DIF_Mat.T_RollUpDoor_C_Yellow_DIF_Mat" :!type "MaterialInterface Object Reference"))))
    (:`then_1`
      (if (`self.IsDoorOpened`)
        (set `self.IsDoorOpened` true)
        (`SceneComponent.K2_SetRelativeLocation` (`self.DoorMesh`) (1.275385 0.0 252.822249) false false)
        (else
          (set `self.IsDoorOpened` false)
          (`SceneComponent.K2_SetRelativeLocation` (`self.DoorMesh`) (1.275385 0.0 -1e-06) false false))))))