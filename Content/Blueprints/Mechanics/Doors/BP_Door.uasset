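; Rotating door with a selectable color variant, toggled directly or by power and scan-completion events.
; ToggleDoor flips the open state, plays a metal sound and swings the mesh with MoveComponentTo, ignoring retriggers while moving.
; Poweron, PowerOff and ScanningFinished set IsPowered, then run the same toggle, which never checks that flag.
; The construction script applies the DoorType material to frame and door and poses the initial open or closed rotation.
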(event `ToggleDoor`
  (if (not (`self.IsOpeningDoor`)) :!label _label
    (set `self.IsOpeningDoor` true)
    (bind _output_get (set `self.IsDoorOpened` (not (`self.IsDoorOpened`))))
    (`GameplayStatics.PlaySoundAtLocation` "/Game/Sounds/Doors/Metal/SW_Door_Metal_Rotating_01_Cue.SW_Door_Metal_Rotating_01_Cue" (`self.K2_GetActorLocation`) (struct) 1.0 1.0 0.0 null null null null)
    (`KismetSystemLibrary.MoveComponentTo` (`self.DoorMesh`) (-56.498962 0.0 0.0) (`KismetMathLibrary.MakeRotator` 0.0 0.0 (select `bool` _output_get :`true` (`self.DoorMaxRotation`))) false false 1.0 true)
    (set `self.IsOpeningDoor` false)))

(event `/Game/Blueprints/BP_Cable/BPI_PowerNew.PowerOn`
  (set `self.IsPowered?` true)
  (goto _label))

(event `/Game/Blueprints/BP_Cable/BPI_PowerNew.PowerOff`
  (set `self.IsPowered?` false)
  (goto _label))

(event `/Game/Blueprints/Mechanics/BlueHandScanner/BPI_HandScannerEvent.ScanningFinished`
  (set `self.IsPowered?` true)
  (goto _label))

(fn `UserConstructionScript`
  (bind _doormesh (`self.DoorMesh`))
  (`|ExecutionSequence`
    (:`then_0`
      (for _array_element (`|MakeArray` (`self.FrameMesh`) (`self.DoorMesh`))
        (`PrimitiveComponent.SetMaterial` _array_element 0 (select `int` (`self.DoorType`) :`0` "/Game/Textures/Kits/Doors/T_Door_A_Blue_DIF_Mat.T_Door_A_Blue_DIF_Mat" :`1` "/Game/Textures/Kits/Doors/T_Door_A_Grey_DIF_Mat.T_Door_A_Grey_DIF_Mat" :`2` "/Game/Textures/Kits/Doors/T_Door_A_Red_DIF_Mat.T_Door_A_Red_DIF_Mat" :`3` "/Game/Textures/Kits/Doors/T_Door_A_Yellow_DIF_Mat.T_Door_A_Yellow_DIF_Mat" :!type "MaterialInterface Object Reference"))))
    (:`then_1`
      (if (`self.IsDoorOpened`)
        (`SceneComponent.K2_SetRelativeRotation` _doormesh (struct :`Yaw` -100.0) false false)
        (else
          (`SceneComponent.K2_SetRelativeRotation` :`self` _doormesh))))))