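; BP_Lever is a lever actor whose switch model is posed open or closed by the construction script from IsOpened.
; BeginPlay caches the player character, but its opening, cancel and hand-visibility events are empty stubs.
; Disconnected logic remains for showing hand meshes, attaching the player's cable, animating the switch by timeline and messaging a linked actor after a delay.
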(event `self.ReceiveBeginPlay`
  (bind _asbp_third_person_character (cast `/Game/ThirdPerson/Blueprints/BP_ThirdPersonCharacter` (`GameplayStatics.GetPlayerCharacter` 0)))
  (set `self.PlayerRef` _asbp_third_person_character))

(event `Opening`)

(event `CancelledOpening`)

(event `SetVisibility_AllHandsOFF`)

(event `SetVisibility_BlueON`)

(event `SetVisibility_RocketON`)

(event `SetVisibility_BlueOFF`)

(event `SetVisibility_RocketOFF`)

(fn `UserConstructionScript`
  (bind _switchmodel (`self.SwitchModel`))
  (`|ExecutionSequence`
    (:`then_0`
      (if (`self.IsOpened?`)
        (`SceneComponent.K2_SetRelativeLocationAndRotation` _switchmodel (0.0 5.567757 13.965023) (struct :`Roll` 40.0) false false)
        (else
          (`SceneComponent.K2_SetRelativeLocationAndRotation` _switchmodel (0.0 5.567757 13.965023) (struct :`Roll` -40.0) false false))))))