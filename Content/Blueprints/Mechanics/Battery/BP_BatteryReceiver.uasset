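; Battery socket actor that, once powered, signals its target door actor and an optional linked actor.
; On overlap it checks the character's inventory for its receiver number, shows a use prompt and registers with the character.
; TurnPowerOn slides the battery in, applies item-colored dynamic emissive materials, plays sounds and sends the messages.
; Construction script presets powered and door state from HaveBatteryIn; BeginPlay auto-powers based on saved opened-door count.
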(event `SetDoorOpened`
  (message `/Game/Blueprints/Mechanics/Battery/BPI_BatteryEvent.Door_SetDoorOpened` (`self.ActorToWith`)))

(event `SetDoorClosed`
  (message `/Game/Blueprints/Mechanics/Battery/BPI_BatteryEvent.Door_SetDoorClosed` (`self.ActorToWith`)))

(event `TurnPowerOn`
  (bind _returnvalue (`self.K2_GetActorLocation`))
  (bind _linkedactor (`self.LinkedActor`))
  (bind _batterymodel (`self.BatteryModel`))
  (bind (_itemname _itemno _itemcolor) (break `/Game/Blueprints/Core/S_ItemData` (`/Game/Blueprints/Core/BP_ItemInfo.ItemData` (`self.MyItemData`))))
  (`Widget.RemoveFromParent` (stale `self.ReceiveActorBeginOverlap` _returnvalue))
  (set `self.HaveBatteryIn?` true)
  (set `self.Powered` true)
  (bind _returnvalue_2 (`KismetMaterialLibrary.CreateDynamicMaterialInstance` "/Game/Textures/Kits/Battery/T_BatteryFrame_DIF_Powered_Mat.T_BatteryFrame_DIF_Powered_Mat"))
  (`MaterialInstanceDynamic.SetVectorParameterValue` _returnvalue_2 "Emissive" _itemcolor)
  (`MaterialInstanceDynamic.SetScalarParameterValue` _returnvalue_2 "Intensity" 1.0)
  (`PrimitiveComponent.SetMaterial` (`self.BatteryReceiverMesh`) 0 _returnvalue_2)
  (`SceneComponent.SetVisibility` _batterymodel true false)
  (bind _returnvalue_3 (`KismetMaterialLibrary.CreateDynamicMaterialInstance` "/Game/Textures/Kits/Battery/T_Battery_DIF_Mat.T_Battery_DIF_Mat"))
  (`MaterialInstanceDynamic.SetVectorParameterValue` _returnvalue_3 "Emissive" _itemcolor)
  (`PrimitiveComponent.SetMaterial` _batterymodel 0 _returnvalue_3)
  (`|ExecutionSequence`
    (:`then_0`
      (`KismetSystemLibrary.MoveComponentTo` _batterymodel (0.0 15.428716 42.777065) (struct :`Roll` 90.0) false false 0.6))
    (:`then_1`
      (`GameplayStatics.PlaySoundAtLocation` "/Game/Sounds/Grabpack/Battery/SW_Battery_PowerOn_01_Cue.SW_Battery_PowerOn_01_Cue" _returnvalue (struct) 1.0 1.0 0.0 null null null null)
      (`GameplayStatics.PlaySoundAtLocation` "/Game/Sounds/Grabpack/Battery/SW_Battery_LockIn_01_Cue.SW_Battery_LockIn_01_Cue" _returnvalue (struct) 1.0 1.0 0.0 null null null null)
      (bind _returnvalue_4 (`AddComponent|NODE_AddAudioComponent-0`))
      (bind _output_get (set `self.SW_IdleSound` _returnvalue_4))
      (`AudioComponent.Play` _output_get 0.0))
    (:`then_2`
      (message `/Game/Blueprints/Mechanics/Battery/BPI_BatteryEvent.BatteryIn` (`self.ActorToWith`))
      (`/Engine/EditorBlueprintResources/StandardMacros.IsValid` _linkedactor
        (:`Is Valid`
          (message `/Game/Blueprints/BP_Cable/BPI_PowerNew.PowerOn` _linkedactor))))))

(event `self.ReceiveActorBeginOverlap`
  (params (OtherActor :type "Actor Object Reference"))
  (if (not (`self.Powered`))
    (bind _asbp_character_1 (cast `/Game/ThirdPerson/Blueprints/BP_Character1` OtherActor))
    (bind _success (`/Game/Blueprints/Core/BPC_Inventory.CheckItem` (`/Game/ThirdPerson/Blueprints/BP_Character1.InventoryComp` _asbp_character_1) (`self.RecieverNumber`)))
    (if _success
      (bind _returnvalue (`|CreateWidget` "/Game/UI/ItemGetUse.ItemGetUse_C"))
      (`UserWidget.AddToViewport` _returnvalue 0)
      (`Widget.SetVisibility` (`/Game/UI/ItemGetUse.Insert` _returnvalue) "Visible")
      (message `/Game/Blueprints/Items/BPI_InteractItem.OverlapForUseItem` OtherActor self))))

(event `self.ReceiveActorEndOverlap`
  (params (OtherActor :type "Actor Object Reference"))
  (`Widget.RemoveFromParent` (stale `self.ReceiveActorBeginOverlap` _returnvalue))
  (message `/Game/Blueprints/Items/BPI_InteractItem.OverlapForUseItem` (stale `self.ReceiveActorBeginOverlap` OtherActor) null))

(event `self.ReceiveBeginPlay`
  (bind _asbp_gi (cast `/Game/Blueprints/Core/BP_GI` (`GameplayStatics.GetGameInstance`)))
  (if (>= (`/Game/Blueprints/Core/BP_SaveGame.Count_OpenedDoor` (`/Game/Blueprints/Core/BP_GI.SaveRef` _asbp_gi)) 2)
    (`self.TurnPowerOn`)))

(fn `UserConstructionScript`
  (bind _batterymodel (`self.BatteryModel`))
  (if (`self.HaveBatteryIn?`)
    (`SceneComponent.SetVisibility` _batterymodel true false)
    (set `self.Powered` true)
    (`PrimitiveComponent.SetMaterial` (`self.BatteryReceiverMesh`) 0 "/Game/Textures/Kits/Battery/T_BatteryFrame_DIF_Powered_Mat.T_BatteryFrame_DIF_Powered_Mat")
    (`self.SetDoorOpened`)
    (else
      (`SceneComponent.SetVisibility` _batterymodel false false)
      (set `self.Powered` false)
      (bind _returnvalue (`KismetMaterialLibrary.CreateDynamicMaterialInstance` "/Game/Textures/Kits/Battery/T_BatteryFrame_DIF_Powered_Mat.T_BatteryFrame_DIF_Powered_Mat"))
      (`MaterialInstanceDynamic.SetVectorParameterValue` _returnvalue "Emissive" (`.ItemColor_12_19B41675494FF60BCB6164A8F51FF42A` (break `/Game/Blueprints/Core/S_ItemData` (`/Game/Blueprints/Core/BP_ItemInfo.ItemData` (`self.MyItemData`)))))
      (`MaterialInstanceDynamic.SetScalarParameterValue` _returnvalue "Intensity" 0.04)
      (`PrimitiveComponent.SetMaterial` (`self.BatteryReceiverMesh`) 0 _returnvalue)
      (`self.SetDoorClosed`))))