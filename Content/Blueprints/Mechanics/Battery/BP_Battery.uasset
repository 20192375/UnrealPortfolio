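; Battery world item that can be interacted with and destroys itself when that happens.
; On BeginPlay it reads the save reference from BP_GI and removes itself if the saved opened-door count has reached a threshold.
; The construction script creates a dynamic material for the battery mesh, setting its emissive color from the item color in its item data.
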(event `self.ReceiveBeginPlay`
  (bind _asbp_gi (cast `/Game/Blueprints/Core/BP_GI` (`GameplayStatics.GetGameInstance`)))
  (if (>= (`/Game/Blueprints/Core/BP_SaveGame.Count_OpenedDoor` (`/Game/Blueprints/Core/BP_GI.SaveRef` _asbp_gi)) 2)
    (`self.K2_DestroyActor`)))

(event `/Game/Characters/BPI_Interact.Interaction`
  (`self.K2_DestroyActor`))

(fn `UserConstructionScript`
  (bind _returnvalue (`KismetMaterialLibrary.CreateDynamicMaterialInstance` "/Game/Textures/Kits/Battery/T_Battery_DIF_Mat.T_Battery_DIF_Mat"))
  (`MaterialInstanceDynamic.SetVectorParameterValue` _returnvalue "Emissive" (`.ItemColor_12_19B41675494FF60BCB6164A8F51FF42A` (break `/Game/Blueprints/Core/S_ItemData` (`/Game/Blueprints/Core/BP_ItemInfo.ItemData` (`self.MyItemData`)))))
  (`PrimitiveComponent.SetMaterial` (`self.BatteryMesh`) 0 _returnvalue))