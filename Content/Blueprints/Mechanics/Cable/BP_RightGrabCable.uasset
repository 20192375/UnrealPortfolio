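; BP_RightGrabCable is a cable actor that draws a mesh cable between two world locations.
; Its MakeSpline event rebuilds CableSpline as two world-space points, then adds a new SplineMesh component stretched between them using the spline's tangents and applies MeshMaterial.
; Earlier spline mesh components are never removed, and a debug print shows each new one's name.
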(event `self.ReceiveBeginPlay`)

(event `self.ReceiveActorBeginOverlap`
  (params (OtherActor :type "Actor Object Reference")))

(event `MakeSpline`
  (params (StartLocation :type "Vector Structure") (EndLocation :type "Vector Structure"))
  (bind _cablespline (`self.CableSpline`))
  (bind _splinemesh (`self.SplineMesh`))
  (bind (_location _tangent) (`SplineComponent.GetLocationAndTangentAtSplinePoint` _cablespline 0 "World"))
  (bind (_location_2 _tangent_2) (`SplineComponent.GetLocationAndTangentAtSplinePoint` _cablespline 1 "World"))
  (`SplineComponent.ClearSplinePoints` _cablespline true)
  (`SplineComponent.AddSplinePointAtIndex` _cablespline StartLocation 0 "World" true)
  (`SplineComponent.AddSplinePointAtIndex` _cablespline EndLocation 1 "World" true)
  (bind _returnvalue (`AddComponent|NODE_AddSplineMeshComponent-0`))
  (bind _output_get (set `self.SplineMesh` _returnvalue))
  (`SplineMeshComponent.SetStartAndEnd` _output_get _location _tangent _location_2 _tangent_2 true)
  (`PrimitiveComponent.SetMaterial` _splinemesh 0 (`self.MeshMaterial`))
  (`KismetSystemLibrary.PrintString` (`KismetSystemLibrary.GetDisplayName` _splinemesh)))

(fn `UserConstructionScript`)